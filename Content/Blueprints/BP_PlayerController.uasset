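; Player controller that owns the main UI widget and handles speed-change input for the third-person character.
; On BeginPlay it creates a hidden WBP_Main, binds its close event and caches the BP_ThirdPersonCharacter.
; Toggling the UI also switches the mouse cursor and disables or re-enables input on the character.
; Speed keys scale the character's current speed up or down multiplicatively, or reset it through the character's own functions.
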(event EventBeginPlay
  (CallFunction|Init))

(event Input|ActionEvents|InputActionToggleMouse
  (params (Key :type Key%20Structure :default "None"))
  (:Pressed
    (UI|ToggleMainUI)))

(event Input|ActionEvents|InputActionSpeedUp
  (params (Key :type Key%20Structure :default "None"))
  (:Pressed
    (Speed|SpeedUp)))

(event Input|ActionEvents|InputActionSpeedDown
  (params (Key :type Key%20Structure :default "None"))
  (:Pressed
    (Speed|SpeedDown)))

(event Input|ActionEvents|InputActionResetSpeed
  (params (Key :type Key%20Structure :default "None"))
  (:Pressed
    (Speed|ResetSpeed)))

(fn ConstructionScript)

(fn Init
  (Utilities|FlowControl|Sequence
    (:then_0
      ;[1 1 1] 构造主界面
      (bind _returnvalue (UserInterface|CreateWidget "/Game/Blueprints/Hud/WBP_Main.WBP_Main_C"))
      (bind _output_get (Variables|Default|SetMainUI _returnvalue))
      (UserInterface|Viewport|AddtoViewport _output_get 0)
      (Widget|SetVisibility (Variables|Default|GetMainUI) "Hidden")
      (EventDispatchers|BindEventtoOnClose (Variables|Default|GetMainUI) (EventDispatchers|CreateEvent :!event OnMainUIClose)))
    (:then_1
      ;[1 1 1] 获得控制的对象
      (bind _asbp_third_person_character (Utilities|Casting|CastToBP_ThirdPersonCharacter (Game|GetPlayerCharacter 0)))
      (Variables|Default|SetMyCharacter _asbp_third_person_character))))

(fn SetMainUIVisible
  (params (Visible :type Boolean))
  (bind _returnvalue (Game|GetPlayerCharacter 0))
  (bind _mainui (Variables|Default|GetMainUI))
  (LocalVariables|SetCurrentVisible Visible)
  (Utilities|FlowControl|Sequence
    (:then_0
      ;[1 1 1] 设定界面是否显示
      (if (LocalVariables|GetCurrentVisible)
        (Widget|SetVisibility _mainui "Visible")
        (else
          (Widget|SetVisibility _mainui "Hidden"))))
    (:then_1
      ;[1 1 1] 设定鼠标是否显示
      (Variables|Default|SetbShowMouseCursor self (LocalVariables|GetCurrentVisible)))
    (:then_2
      ;[1 1 1] 设定是否禁用玩家输入
      (if (LocalVariables|GetCurrentVisible)
        (Input|DisableInput _returnvalue 0)
        (else
          (Input|EnableInput _returnvalue 0))))))

(fn ToggleMainUI
  (UI|SetMainUIVisible (not (Widget|IsVisible (Variables|Default|GetMainUI)))))

(fn OnMainUIClose
  (UI|SetMainUIVisible false))

(fn SpeedUp
  (bind _mycharacter (Variables|Default|GetMyCharacter))
  (bind _speed (Default|GetSpeed _mycharacter))
  (Default|SetSpeed _mycharacter (* _speed 1.5)))

(fn SpeedDown
  (bind _mycharacter (Variables|Default|GetMyCharacter))
  (bind _speed (Default|GetSpeed _mycharacter))
  (Default|SetSpeed _mycharacter (* _speed 0.75)))

(fn ResetSpeed
  (Default|ResetSpeed (Variables|Default|GetMyCharacter)))