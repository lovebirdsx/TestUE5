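; BP_StateComponent is a component that stores state as key-value pairs in StateMap, with Get and Contains for lookup.
; Set always writes and fires StateSeted, while Change writes and fires StateChanged only if the key is missing or its value differs.
; Remove deletes the key and always fires StateRemoved, and Get returns an empty value for missing keys.
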(event EventBeginPlay)

(event EventTick
  (params (DeltaSeconds :type Float%20%28single-precision%29)))

(fn Set
  (params (Key :type String) (Value :type String))
  (Utilities|Map|Add (Variables|Default|GetStateMap) Key Value)
  (Default|CallStateSeted Key Value))

(fn Remove
  (params (Key :type String))
  (Utilities|Map|Remove (Variables|Default|GetStateMap) Key)
  (Default|CallStateRemoved Key))

(fn Change
  (params (Key :type String) (Value :type String))
  (bind _statemap (Variables|Default|GetStateMap))
  (bind (_value _returnvalue) (Utilities|Map|Find _statemap Key))
  (if (not (and (Utilities|Enum|Equal(Enum) Value _value) _returnvalue))
    (Utilities|Map|Add (Variables|Default|GetStateMap) Key Value)
    (Default|CallStateChanged Key Value)))

(fn Get
  (params (Key :type String))
  (bind _statemap (Variables|Default|GetStateMap))
  (bind (_value _returnvalue) (Utilities|Map|Find _statemap Key))
  (if _returnvalue
    (return _value)
    (else
      (return ""))))

(fn Contains
  (params (Key :type String))
  (return (Utilities|Map|Contains (Variables|Default|GetStateMap) Key)))