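; BP_Screen is an entity that displays a text value from its state on a TextRender component.
; It listens to the state component's set and change events and, when the key is "Screen", converts the value to text and shows it.
; BeginPlay and construction only call the parent, and SetDoorState is an empty stub.
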(event StateSeted(BP_StateComponent)
  (params (Key :type String) (Value :type String))
  (if (Utilities|Enum|Equal(Enum) Key "Screen")
    (Rendering|Components|TextRender|SetText (Variables|Default|GetTextRender) (Utilities|Text|ToText(String) Value))))

(event StateChanged(BP_StateComponent)
  (params (Key :type String) (Value :type String))
  (if (Utilities|Enum|Equal(Enum) Key "Screen")
    (Rendering|Components|TextRender|SetText (Variables|Default|GetTextRender) (Utilities|Text|ToText(String) Value))))

(event EventBeginPlay
  (|CallParentFunction))

(fn ConstructionScript
  (|CallParentFunction))

(fn SetDoorState
  (params (IsOpen :type Boolean)))