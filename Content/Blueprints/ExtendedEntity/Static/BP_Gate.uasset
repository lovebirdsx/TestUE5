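; BP_Gate is a sliding gate entity that opens and closes according to the "ActorState" key of its BP_StateComponent.
; The construction script records GateLeft's start position and derives the open position by adding OpenOffset along local Y.
; StateSeted snaps GateLeft instantly to either position, while StateChanged animates it over OpenTime with MoveComponentTo and prints unknown states.
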(event StateSeted(BP_StateComponent)
  (params (Key :type String) (Value :type String))
  (if (Utilities|Enum|Equal(Enum) Key "ActorState")
    (switch string Value
      (:Open
        (CallFunction|SetDoorState true))
      (:Close
        (CallFunction|SetDoorState false)))))

(event StateChanged(BP_StateComponent)
  (params (Key :type String) (Value :type String))
  (if (Utilities|Enum|Equal(Enum) Key "ActorState")
    (switch string Value
      (:Default
        (Development|PrintString (Utilities|String|ToString(Text) (Utilities|Text|FormatText "Unknown State {State}" Value))))
      (:Open
        (Components|MoveComponentTo (Variables|Default|GetGateLeft) (Variables|Default|GetEndPos) "0, 0, 0" false false (Variables|Default|GetOpenTime) false))
      (:Close
        (Components|MoveComponentTo (Variables|Default|GetGateLeft) (Variables|Default|GetStartPos) "0, 0, 0" false false (Variables|Default|GetOpenTime) false)))))

(event EventBeginPlay
  (|CallParentFunction))

(fn ConstructionScript
  (|CallParentFunction)
  (bind _output_get (Variables|Default|SetStartPos (Variables|/Script/Engine.SceneComponent|GetRelativeLocation (Variables|Default|GetGateLeft))))
  (Variables|Default|SetEndPos (Math|Vector|MakeVector (.x _output_get) (+ (.y _output_get) (Variables|Default|GetOpenOffset)) (.z _output_get))))

(fn SetDoorState
  (params (IsOpen :type Boolean))
  (if IsOpen
    (Transformation|SetRelativeLocation (Variables|Default|GetGateLeft) (Variables|Default|GetEndPos) false false)
    (else
      (Transformation|SetRelativeLocation (Variables|Default|GetGateLeft) (Variables|Default|GetStartPos) false false))))