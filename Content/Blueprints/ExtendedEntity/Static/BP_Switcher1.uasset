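; BP_Switcher1 is a switcher entity whose sphere glows according to its Open or Close state.
; The construction script creates a dynamic material instance on the sphere.
; State component events for "ActorState" play or reverse a timeline that scales Glow up to MaxGlow, and StateChanged reports unknown values as errors.
; SetSwicherState sets the glow instantly to full or zero, but nothing in this file calls it.
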(event StateSeted(BP_StateComponent)
  (params (Key :type String) (Value :type String))
  (if (Utilities|Enum|Equal(Enum) Key "ActorState")
    (switch string Value
      (:Open
        (bind _glow (Timeline|Timeline_0 Play)
          (:Update
            (Rendering|Material|SetScalarParameterValue (Variables|Material|GetMaterial) "Glow" (* _glow (Variables|Material|GetMaxGlow)) :!class /Script/Engine.MaterialInstanceDynamic))))
      (:Close
        (Timeline|Timeline_0 Reverse)))))

(event StateChanged(BP_StateComponent)
  (params (Key :type String) (Value :type String))
  (if (Utilities|Enum|Equal(Enum) Key "ActorState")
    (switch string Value
      (:Default
        (Class|MyLog|Error (Utilities|String|ToString(Text) (Utilities|Text|FormatText "Unknown State {State}" Value))))
      (:Open
        (bind _glow (Timeline|Timeline_0 Play)
          (:Update
            (Rendering|Material|SetScalarParameterValue (Variables|Material|GetMaterial) "Glow" (* _glow (Variables|Material|GetMaxGlow)) :!class /Script/Engine.MaterialInstanceDynamic))))
      (:Close
        (Timeline|Timeline_0 Reverse)))))

(event EventBeginPlay
  (|CallParentFunction) ; This node is disabled and will not be called.\nDrag off pins to build functionality.
)

(event Collision|EventActorBeginOverlap
  (params (OtherActor :type Actor%20Object%20Reference))
  (|CallParentFunction OtherActor) ; This node is disabled and will not be called.\nDrag off pins to build functionality.
)

(event EventTick
  (params (DeltaSeconds :type Float%20%28single-precision%29)))

(fn ConstructionScript
  (|CallParentFunction)
  (bind _returnvalue (Rendering|Material|CreateDynamicMaterialInstance (Variables|Components|GetSphere) 0 "/Game/Demo/Meterials/M_Swicher_Inst.M_Swicher_Inst" "Switcher" :!class /Script/Engine.PrimitiveComponent))
  (Variables|Material|SetMaterial _returnvalue))

(fn SetSwicherState
  (params (IsOn :type Boolean))
  (bind _material (Variables|Material|GetMaterial))
  (if IsOn
    (Rendering|Material|SetScalarParameterValue _material "Glow" (Variables|Material|GetMaxGlow) :!class /Script/Engine.MaterialInstanceDynamic)
    (else
      (Rendering|Material|SetScalarParameterValue _material "Glow" 0.0 :!class /Script/Engine.MaterialInstanceDynamic))))