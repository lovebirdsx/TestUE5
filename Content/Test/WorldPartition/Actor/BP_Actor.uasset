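; BP_Actor is a test actor in the World Partition test folder that reports its lifecycle with printed messages.
; BeginPlay and EndPlay each call their own function, which formats the actor's display name into a begin or end play message and prints it.
; The construction script is empty, and the actor has no other logic.
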(event EventBeginPlay
  (CallFunction|OnBeginPlay))

(event EventEndPlay
  (params (EndPlayReason :type EEndPlayReason%20Enum :default "Destroyed"))
  (CallFunction|OnEndPlay1))

(fn ConstructionScript)

(fn OnBeginPlay
  (Development|PrintText (Utilities|Text|FormatText "{actor} begion play" (Utilities|GetDisplayName self))))

(fn OnEndPlay1
  (Development|PrintText (Utilities|Text|FormatText "{actor} end play" (Utilities|GetDisplayName self))))