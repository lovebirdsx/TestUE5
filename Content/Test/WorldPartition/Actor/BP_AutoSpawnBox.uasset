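; BP_AutoSpawnBox is a World Partition test actor that replaces its four sphere marker components with spawned actors on BeginPlay.
; Each sphere's world location feeds SpawnByEditor, which spawns at a fixed rotation and unit scale, then the sphere is destroyed.
; AutoSetOwner selects between a spawn owned by this actor, with no class shown, and an unowned BP_Box.
; SpawnByGame duplicates SpawnByEditor's logic but is not called here.
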(event EventBeginPlay
  (Utilities|FlowControl|Sequence
    (:then_0
      (CallFunction|SpawnActorandDestroyMesh (Variables|Default|GetSphere1)))
    (:then_1
      (CallFunction|SpawnActorandDestroyMesh (Variables|Default|GetSphere2)))
    (:then_2
      (CallFunction|SpawnActorandDestroyMesh (Variables|Default|GetSphere3)))
    (:then_3
      (CallFunction|SpawnActorandDestroyMesh (Variables|Default|GetSphere4)))))

(fn ConstructionScript
  (|CallParentFunction))

(fn SpawnActorandDestroyMesh
  (params (Component :type Static%20Mesh%20Component%20Object%20Reference))
  (CallFunction|SpawnbyEditor (Transformation|GetWorldTransform Component))
  (Components|DestroyComponent Component))

(fn SpawnbyEditor
  (params (Transform :type Transform))
  (bind _returnvalue (Math|Transform|TransformLocation Transform "0, 0, 0"))
  (bind _returnvalue_2 (Math|Transform|MakeTransform _returnvalue "45.000000, 0, 0"))
  (if (Variables|Default|GetAutoSetOwner)
    (Game|SpawnActorfromClass "/Game/Test/WorldPartition/Actor/BP_Box.BP_Box_C" _returnvalue_2 "Undefined" self 0)
    (else
      (Game|SpawnActorfromClass "/Game/Test/WorldPartition/Actor/BP_Box.BP_Box_C" _returnvalue_2 "Undefined" 0 0))))

(fn SpawnbyGame
  (params (Transform :type Transform))
  (bind _returnvalue (Math|Transform|TransformLocation Transform "0, 0, 0"))
  (bind _returnvalue_2 (Math|Transform|MakeTransform _returnvalue "45.000000, 0, 0"))
  (if (Variables|Default|GetAutoSetOwner)
    (Game|SpawnActorfromClass "/Game/Test/WorldPartition/Actor/BP_Box.BP_Box_C" _returnvalue_2 "Undefined" self 0)
    (else
      (Game|SpawnActorfromClass "/Game/Test/WorldPartition/Actor/BP_Box.BP_Box_C" _returnvalue_2 "Undefined" 0 0))))